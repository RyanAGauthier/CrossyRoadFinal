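; BP_Eagle is an eagle hazard that swoops at the chicken player and simulates grabbing it.
; It plays a spawn sound, then moves every Tick along local Y and Z using EagleSpeed.
; On first capsule overlap with BP_Player, it scales the player's mesh and capsule to zero rather than attaching them.
; It also reverses its vertical speed, sets a one-time grab flag and plays hit and death sounds.
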(event OnComponentBeginOverlap(Capsule)
  (params (OverlappedComponent :type Primitive%20Component%20Object%20Reference) (OtherActor :type Actor%20Object%20Reference) (OtherComp :type Primitive%20Component%20Object%20Reference) (OtherBodyIndex :type Integer) (bFromSweep :type Boolean) (SweepResult :type Hit%20Result%20Structure%20%28by%20ref%29))
  (bind _asbp_player (Utilities|Casting|CastToBP_Player OtherActor))
  (if (not (Variables|Default|GetGrabbedPlayer))
    (Transformation|SetRelativeScale3D (Variables|/Game/BluePrints/BP_Player.BP_Player_C|GetChickenMesh _asbp_player) "0, 0, 0")
    (Transformation|SetRelativeScale3D (Variables|/Game/BluePrints/BP_Player.BP_Player_C|GetCapsule _asbp_player) "0, 0, 0")
    (Variables|Default|SetEagleSpeed (Math|Vector|MakeVector (.x (Variables|Default|GetEagleSpeed)) (.y (Variables|Default|GetEagleSpeed)) (* (.z (Variables|Default|GetEagleSpeed)) -1.0)))
    (Variables|Default|SetGrabbedPlayer true)
    (Audio|PlaySound2D "/Game/Sounds/eaglehit.eaglehit" 1.0 1.0 0.0 0 0)
    (Audio|PlaySound2D "/Game/Sounds/ChickenDeathKnell.ChickenDeathKnell" 1.0 1.0 0.0 0 0)))

(event EventBeginPlay
  (Audio|PlaySoundatLocation "/Game/Sounds/EagleSpawned.EagleSpawned" (Transformation|GetActorLocation) "0, 0, 0" 1.0 1.0 0.0 0 0 0))

(event Collision|EventActorBeginOverlap
  (params (OtherActor :type Actor%20Object%20Reference)))

(event EventTick
  (params (DeltaSeconds :type Float%20%28single-precision%29))
  (bind _eaglespeed (Variables|Default|GetEagleSpeed))
  (Transformation|AddActorLocalOffset (Math|Vector|MakeVector 0.0 (* DeltaSeconds (* (.x _eaglespeed) -1.0)) (* (/ (.z _eaglespeed) -1.0) DeltaSeconds)) false false))

(fn ConstructionScript)