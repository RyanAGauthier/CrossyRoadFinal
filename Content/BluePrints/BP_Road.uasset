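; BP_Road is a traffic lane actor that spawns a stream of cars or trucks, depending on VehicleToSpawn, with a rare chance of a coin along it.
; After a short random delay it spawns the first vehicle, then Tick spawns another whenever the last one has moved CarGap away along Y.
; A VehicleDeathZone overlap destroys cars and trucks at the lane's end, and destroying the road cleans up its coin and spawned vehicles.
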(event OnComponentBeginOverlap(VehicleDeathZone)
  (params (OverlappedComponent :type Primitive%20Component%20Object%20Reference) (OtherActor :type Actor%20Object%20Reference) (OtherComp :type Primitive%20Component%20Object%20Reference) (OtherBodyIndex :type Integer) (bFromSweep :type Boolean) (SweepResult :type Hit%20Result%20Structure%20%28by%20ref%29))
  (Utilities|Casting|CastToBP_Bluecar OtherActor
    (:then
      _)
    (:CastFailed
      (Utilities|Casting|CastToBP_Truck OtherActor)))
  (Actor|DestroyActor OtherActor))

(event EventBeginPlay
  (bind _returnvalue (Transformation|GetActorLocation))
  (bind _returnvalue_2 (Transformation|GetActorLocation))
  (bind _vehicletospawn (Variables|Default|GetVehicleToSpawn))
  (if (== (Math|Random|RandomInteger 50) 49)
    (if (> (.y (Transformation|GetActorLocation)) 0.0)
      (Variables|Default|SetCoinSpacing -9e+01))
    (bind _returnvalue_3 (Game|SpawnActorfromClass "/Game/BluePrints/BP_Simplecoin.BP_Simplecoin_C" (Math|Transform|MakeTransform (Math|Vector|MakeVector (.x _returnvalue) (+ (.y _returnvalue) (* (Math|Random|RandomInteger 23) (Variables|Default|GetCoinSpacing))) (+ (.z _returnvalue) 2e+01)) "0, 0, 0" "1,1,1") "Undefined" 0 0))
    (Variables|Default|SetMyCoin _returnvalue_3))
  (Utilities|FlowControl|Delay (Math|Random|RandomFloatinRange 0.0 0.5))
  (Variables|Default|SetTimeToGo true)
  (if (Utilities|Enum|Equal(Enum) _vehicletospawn "Car")
    (CallFunction|SpawnCar _returnvalue_2 (Variables|Default|GetLaneSpeed) (Variables|Default|GetOrientation))
    (elif (Utilities|Enum|Equal(Enum) _vehicletospawn "Truck")
      (CallFunction|SpawnTruck _returnvalue_2 (Variables|Default|GetLaneSpeed) (Transformation|GetActorRotation)))))

(event Collision|EventActorBeginOverlap
  (params (OtherActor :type Actor%20Object%20Reference)))

(event EventTick
  (params (DeltaSeconds :type Float%20%28single-precision%29))
  (bind _orientation (Variables|Default|GetOrientation))
  (bind _vehicletospawn (Variables|Default|GetVehicleToSpawn))
  (if (Variables|Default|GetTimeToGo)
    (if (Utilities|Enum|Equal(Enum) _vehicletospawn "Car")
      (if (>= (Math|Float|Absolute(Float) (- (.y (Transformation|GetActorLocation (Variables|Default|GetLastCarSpawned))) (.y (Transformation|GetActorLocation)))) (Variables|Default|GetCarGap))
        (CallFunction|SpawnCar (Transformation|GetActorLocation) (Variables|Default|GetLaneSpeed) _orientation))
      (elif (Utilities|Enum|Equal(Enum) _vehicletospawn "Truck")
        (if (>= (Math|Float|Absolute(Float) (- (.y (Transformation|GetActorLocation (Variables|Default|GetLastTruckSpawned))) (.y (Transformation|GetActorLocation)))) (Variables|Default|GetCarGap))
          (CallFunction|SpawnTruck (Transformation|GetActorLocation) (Variables|Default|GetLaneSpeed) _orientation))))))

(event EventDestroyed
  (bind _vehicletospawn (Variables|Default|GetVehicleToSpawn))
  (bind _mycoin (Variables|Default|GetMyCoin))
  (Utilities|IsValid _mycoin
    (:Is%20Valid
      (Actor|DestroyActor _mycoin))
    (:Is%20Not%20Valid
      _))
  (if (Utilities|Enum|Equal(Enum) _vehicletospawn "Car")
    (for _array_element (Variables|Default|GetCarArray)
      (Utilities|IsValid _array_element
        (:Is%20Valid
          (Actor|DestroyActor _array_element))))
    (elif (Utilities|Enum|Equal(Enum) _vehicletospawn "Truck")
      (for _array_element_2 (Variables|Default|GetTruckArray)
        (Utilities|IsValid _array_element_2
          (:Is%20Valid
            (Actor|DestroyActor _array_element_2)))))))

(fn ConstructionScript)

(fn SpawnCar
  (params (SpawnLocation :type Vector) (CarSpeed :type Float%20%28single-precision%29) (CarOrientation :type Rotator))
  (bind _returnvalue (Game|SpawnActorfromClass "/Game/BluePrints/BP_Bluecar.BP_Bluecar_C" (Math|Transform|MakeTransform (Math|Vector|MakeVector (.x SpawnLocation) (.y SpawnLocation) (+ (.z SpawnLocation) 2e+01)) CarOrientation "1,1,1") "Undefined" 0 CarSpeed 0))
  (bind _output_get (Variables|Default|SetLastCarSpawned _returnvalue))
  (Utilities|Array|Add (Variables|Default|GetCarArray) _output_get)
  (return _output_get))

(fn SpawnTruck
  (params (SpawnLocation :type Vector) (TruckSpeed :type Float%20%28single-precision%29) (TruckOrientation :type Rotator))
  (bind _returnvalue (Game|SpawnActorfromClass "/Game/BluePrints/BP_Truck.BP_Truck_C" (Math|Transform|MakeTransform (Math|Vector|MakeVector (.x SpawnLocation) (.y SpawnLocation) (+ (.z SpawnLocation) 6e+01)) TruckOrientation "1,1,1") "Undefined" 0 TruckSpeed 0))
  (bind _output_get (Variables|Default|SetLastTruckSpawned _returnvalue))
  (Utilities|Array|Add (Variables|Default|GetTruckArray) _output_get)
  (return _output_get))