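; BP_RailRoad is a railroad actor that repeatedly sends trains along its track and occasionally spawns a coin.
; A timeline replayed from Tick plays a warning sound once per cycle, then spawns a fast BP_Train on finish and resets.
; Trains leaving the Box volume are destroyed.
; BeginPlay rarely places a coin at a random Y offset, tracked with the trains in TrainArray for cleanup when the railroad is destroyed.
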(event OnComponentEndOverlap(Box)
  (params (OverlappedComponent :type Primitive%20Component%20Object%20Reference) (OtherActor :type Actor%20Object%20Reference) (OtherComp :type Primitive%20Component%20Object%20Reference) (OtherBodyIndex :type Integer))
  (bind _asbp_train (Utilities|Casting|CastToBP_Train OtherActor))
  (Actor|DestroyActor _asbp_train))

(event EventBeginPlay
  (bind _returnvalue (Transformation|GetActorLocation))
  (if (== (Math|Random|RandomInteger 50) 49)
    (if (> (.y _returnvalue) 0.0)
      (Variables|Default|SetCoinSpacing -9e+01))
    (bind _returnvalue_2 (Game|SpawnActorfromClass "/Game/BluePrints/BP_Simplecoin.BP_Simplecoin_C" (Math|Transform|MakeTransform (Math|Vector|MakeVector (.x _returnvalue) (+ (.y _returnvalue) (* (Math|Random|RandomInteger 23) (Variables|Default|GetCoinSpacing))) (+ (.z _returnvalue) 2e+01)) "0, 0, 0" "1,1,1") "Undefined" 0 0))
    (Utilities|Array|Add (Variables|Default|GetTrainArray) _returnvalue_2)))

(event Collision|EventActorBeginOverlap
  (params (OtherActor :type Actor%20Object%20Reference)))

(event EventTick
  (params (DeltaSeconds :type Float%20%28single-precision%29))
  (bind _returnvalue (Transformation|GetActorLocation))
  (bind _newtrack_0 (Timeline|Timeline_0 Play)
    (:Update
      (if (and (not (Variables|Default|GetWarnedOfTrain)) (== _newtrack_0 1.0))
        (Audio|PlaySoundatLocation "/Game/Sounds/TrainWarning.TrainWarning" (Math|Vector|MakeVector (.x _returnvalue) 5e+02 (.z _returnvalue)) "0, 0, 0" 1.0 1.0 0.0 0 0 0)
        (Variables|Default|SetWarnedOfTrain true)))
    (:Finished
      (CallFunction|SpawnTrain (Math|Vector|MakeVector (.x _returnvalue) (.y _returnvalue) (.z _returnvalue)) (Transformation|GetActorRotation) 2e+03)
      (Variables|Default|SetWarnedOfTrain false)
      (Timeline|Timeline_0 SetNewTime))))

(event EventDestroyed
  (for _array_element (Variables|Default|GetTrainArray)
    (Utilities|IsValid _array_element
      (:Is%20Valid
        (Actor|DestroyActor _array_element)))))

(fn ConstructionScript)

(fn SpawnTrain
  (params (SpawnLocation :type Vector) (Orientation :type Rotator) (Speed :type Float%20%28single-precision%29))
  (bind _returnvalue (Game|SpawnActorfromClass "/Game/BluePrints/BP_Train.BP_Train_C" (Math|Transform|MakeTransform (Math|Vector|MakeVector (.x SpawnLocation) (.y SpawnLocation) (+ (.z SpawnLocation) 5e+01)) Orientation "1,1,1") "Undefined" 0 Speed 0))
  (Utilities|Array|Add (Variables|Default|GetTrainArray) _returnvalue))