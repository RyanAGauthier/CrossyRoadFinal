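; River actor that fills itself with either lilypads or moving logs, depending on EntityToSpawn.
; In Lilypad mode, BeginPlay randomly fills a row of slots along Y, occasionally adding a coin on a pad.
; In Log mode, Tick spawns a new log once the last is far enough away in Y, and LogDeathZone destroys logs overlapping it.
; Spawned actors are tracked in arrays and destroyed with the river.
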(event OnComponentBeginOverlap(LogDeathZone)
  (params (OverlappedComponent :type Primitive%20Component%20Object%20Reference) (OtherActor :type Actor%20Object%20Reference) (OtherComp :type Primitive%20Component%20Object%20Reference) (OtherBodyIndex :type Integer) (bFromSweep :type Boolean) (SweepResult :type Hit%20Result%20Structure%20%28by%20ref%29))
  (bind _asbp_log (Utilities|Casting|CastToBP_Log OtherActor))
  (Actor|DestroyActor _asbp_log))

(event EventBeginPlay
  (bind _returnvalue (Transformation|GetActorLocation))
  (if (Utilities|Enum|Equal(Enum) (Variables|Default|GetEntityToSpawn) "Lilypad")
    (for _index (range 0 22)
      (if (not (== (Math|Random|RandomInteger 2) 0))
        (CallFunction|SpawnLilypadsandCoins (Math|Vector|MakeVector (.x _returnvalue) (+ (* _index 9e+01) (.y _returnvalue)) (.z _returnvalue)))))
    (else
      (CallFunction|SpawnLog (Transformation|GetActorLocation) (Transformation|GetActorRotation) 7e+01))))

(event Collision|EventActorBeginOverlap
  (params (OtherActor :type Actor%20Object%20Reference)))

(event EventTick
  (params (DeltaSeconds :type Float%20%28single-precision%29))
  (if (Utilities|Enum|Equal(Enum) (Variables|Default|GetEntityToSpawn) "Log")
    (if (>= (Math|Float|Absolute(Float) (- (.y (Transformation|GetActorLocation (Variables|Default|GetLastLogSpawned))) (.y (Transformation|GetActorLocation)))) 2e+02)
      (CallFunction|SpawnLog (Transformation|GetActorLocation) (Transformation|GetActorRotation) 7e+01))))

(event EventDestroyed
  (bind _entitytospawn (Variables|Default|GetEntityToSpawn))
  (if (Utilities|Enum|Equal(Enum) _entitytospawn "Lilypad")
    (for _array_element (Variables|Default|GetMyCoinArray)
      (Utilities|IsValid _array_element
        (:Is%20Valid
          (Actor|DestroyActor _array_element))))
    (for _array_element_2 (Variables|Default|GetLilypadArray)
      (Utilities|IsValid _array_element_2
        (:Is%20Valid
          (Actor|DestroyActor _array_element_2))))
    (elif (Utilities|Enum|Equal(Enum) _entitytospawn "Log")
      (for _array_element_3 (Variables|Default|GetLogArray)
        (Utilities|IsValid _array_element_3
          (:Is%20Valid
            (Actor|DestroyActor _array_element_3)))))))

(fn ConstructionScript)

(fn SpawnLilypadsandCoins
  (params (SpawnLocation :type Vector))
  (bind _returnvalue (+ (.z SpawnLocation) 2e+01))
  (bind _returnvalue_2 (Game|SpawnActorfromClass "/Game/BluePrints/BP_Lilypad.BP_Lilypad_C" (Math|Transform|MakeTransform (Math|Vector|MakeVector (.x SpawnLocation) (.y SpawnLocation) _returnvalue) "0, 0, 0" "1,1,1") "Undefined" 0 0))
  (Utilities|Array|Add (Variables|Default|GetLilypadArray) _returnvalue_2)
  (if (== (Math|Random|RandomInteger 25) 24)
    (bind _returnvalue_3 (Game|SpawnActorfromClass "/Game/BluePrints/BP_Simplecoin.BP_Simplecoin_C" (Math|Transform|MakeTransform (Math|Vector|MakeVector (.x SpawnLocation) (.y SpawnLocation) (+ _returnvalue 1e+01)) "0, 0, 0" "1,1,1") "Undefined" 0 0))
    (Utilities|Array|Add (Variables|Default|GetMyCoinArray) _returnvalue_3)))

(fn SpawnLog
  (params (SpawnLocation :type Vector) (Orientation :type Rotator) (Speed :type Float%20%28single-precision%29))
  (bind _returnvalue (Game|SpawnActorfromClass "/Game/BluePrints/BP_Log.BP_Log_C" (Math|Transform|MakeTransform (Math|Vector|MakeVector (.x SpawnLocation) (.y SpawnLocation) (+ (.z SpawnLocation) 1e+01)) Orientation "1,1,1") "Undefined" 0 Speed 0))
  (bind _output_get (Variables|Default|SetLastLogSpawned _returnvalue))
  (Utilities|Array|Add (Variables|Default|GetLogArray) _output_get))