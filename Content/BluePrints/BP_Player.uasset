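; Player chicken pawn for a Crossy Road-style game, hopping across roads, rails and rivers while collecting coins and scoring forward progress.
; Hop inputs set a target that Tick animates with a timeline, then side probes block moves into trees, rocks and bounds.
; Vehicles, water without footing, three back hops or idling (eagle) cause death.
; Coins and high score load from a save slot and are saved on death before quitting.
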(event OnComponentBeginOverlap(FrontProbe)
  (params (OverlappedComponent :type Primitive%20Component%20Object%20Reference) (OtherActor :type Actor%20Object%20Reference) (OtherComp :type Primitive%20Component%20Object%20Reference) (OtherBodyIndex :type Integer) (bFromSweep :type Boolean) (SweepResult :type Hit%20Result%20Structure%20%28by%20ref%29))
  (bind _isjumping (Variables|Default|GetIsJumping))
  (Utilities|Casting|CastToBP_River OtherActor
    (:then
      (if (not _isjumping) :!label _label
        (Variables|Default|SetChickenHeight 95.0)))
    (:CastFailed
      (Utilities|Casting|CastToBP_Grass OtherActor
        (:then
          (goto _label))
        (:CastFailed
          (Utilities|Casting|CastToBP_Railroad OtherActor
            (:then
              _)
            (:CastFailed
              (Utilities|Casting|CastToBP_Road OtherActor)))
          (if (not _isjumping)
            (Variables|Default|SetChickenHeight 85.0)))))))

(event OnComponentBeginOverlap(Capsule)
  (params (OverlappedComponent :type Primitive%20Component%20Object%20Reference) (OtherActor :type Actor%20Object%20Reference) (OtherComp :type Primitive%20Component%20Object%20Reference) (OtherBodyIndex :type Integer) (bFromSweep :type Boolean) (SweepResult :type Hit%20Result%20Structure%20%28by%20ref%29))
  (if (not (Variables|Default|GetIsDoomed))
    (Utilities|Casting|CastToBP_Bluecar OtherActor
      (:then
        (Variables|Default|SetIsDoomed true)
        (Transformation|SetRelativeScale3D (Variables|Default|GetChickenMesh) "1.000000,1.000000,0.250000" :!label _label)
        (Audio|PlaySound2D "/Game/Sounds/ChickenDeathKnell.ChickenDeathKnell" 1.0 1.0 0.0 0 0)
        (Audio|PlaySound2D "/Game/Sounds/carsquish3.carsquish3" 1.0 1.0 0.0 0 0)
        (Transformation|SetRelativeLocation (Variables|Default|GetChickenMesh) "0, 0,-40.000000" false false)
        (Input|SetInputModeUIOnly (Game|GetPlayerController 0) 0 "DoNotLock" :!label _label_2)
        (Utilities|FlowControl|Delay 3.0)
        (CallFunction|KillChicken)
        (Game|QuitGame 0 "Quit" false))
      (:CastFailed
        (Utilities|Casting|CastToBP_Truck OtherActor
          (:then
            (Variables|Default|SetIsDoomed true)
            (goto _label))
          (:CastFailed
            (Utilities|Casting|CastToBP_Lilypad OtherActor
              (:then
                (Audio|PlaySound2D "/Game/Sounds/HopOnLilypad.HopOnLilypad" 1.0 1.0 0.0 0 0))
              (:CastFailed
                (Utilities|Casting|CastToBP_Train OtherActor
                  (:then
                    (Variables|Default|SetIsDoomed true)
                    (Audio|PlaySound2D "/Game/Sounds/ChickenDeathKnell.ChickenDeathKnell" 1.0 1.0 0.0 0 0)
                    (Audio|PlaySound2D "/Game/Sounds/explosiontemp.explosiontemp" 1.0 1.0 0.0 0 0)
                    (Effects|SpawnEmitteratLocation "/Game/Misc/PS_Test.PS_Test" (Transformation|GetActorLocation))
                    (Transformation|SetWorldScale3D (Variables|Default|GetChickenMesh) "0, 0, 0")
                    (goto _label_2))
                  (:CastFailed
                    (Utilities|Casting|CastToBP_Log OtherActor
                      (:then
                        (Audio|PlaySound2D "/Game/Sounds/HopOnLog.HopOnLog" 1.0 1.0 0.0 0 0))
                      (:CastFailed
                        (bind _asbp_simplecoin (Utilities|Casting|CastToBP_Simplecoin OtherActor))
                        (Audio|PlaySound2D "/Game/Sounds/GetCoin.GetCoin" 1.0 1.0 0.0 0 0)
                        (Actor|DestroyActor _asbp_simplecoin)
                        (Variables|Default|SetCoinsCollected (+ (Variables|Default|GetCoinsCollected) 1))))))))))))))

(event EventBeginPlay
  (bind _returnvalue (SaveGame|LoadGamefromSlot "save"))
  (bind _asbp_savegame (Utilities|Casting|CastToBP_Savegame _returnvalue)
    (:then
      (Development|PrintString "\"Loaded save!\"")
      (bind _output_get (Variables|Default|SetMySave _asbp_savegame))
      (Variables|Default|SetCoinsCollected (Variables|/Game/BluePrints/BP_Savegame.BP_Savegame_C|GetTotalCoins _output_get)))
    (:CastFailed
      (bind _returnvalue_2 (SaveGame|CreateSaveGameObject "/Game/BluePrints/BP_Savegame.BP_Savegame_C"))
      (bind _output_get_2 (Variables|Default|SetMySave _returnvalue_2))
      (Variables|Default|SetCoinsCollected (Variables|/Game/BluePrints/BP_Savegame.BP_Savegame_C|GetTotalCoins _output_get_2))
      (Development|PrintString "\"Created Save\"")))
  (bind _returnvalue_3 (UserInterface|CreateWidget "/Game/Misc/WBP_UI.WBP_UI_C"))
  (UserInterface|Viewport|AddtoViewport _returnvalue_3 0)
  (Variables|/Game/Misc/WBP_UI.WBP_UI_C|SetChicken _returnvalue_3 self)
  (bind _output_get_3 (Variables|Default|SetMyHUD _returnvalue_3))
  (Default|UpdateUI _output_get_3))

(event EventTick
  (params (DeltaSeconds :type Float%20%28single-precision%29))
  (bind _returnvalue (Transformation|GetActorLocation))
  (bind _returnvalue_2 (Transformation|GetActorLocation))
  (bind _chickenendpos (Variables|Default|GetChickenEndPos))
  (bind _capsule (Variables|Default|GetCapsule))
  (Variables|Default|SetTimeUntilEaten (- (Variables|Default|GetTimeUntilEaten) DeltaSeconds))
  (if (Variables|Default|GetIsJumping)
    (bind (_direction _newtrack_0 _newtrack_2) (Timeline|Timeline_0 Play)
      (:Update
        (Transformation|SetWorldLocation (Variables|Default|GetDefaultSceneRoot) (Math|Vector|MakeVector (Math|Float|Lerp (.x (Variables|Default|GetChickenStartPos)) (.x _chickenendpos) _newtrack_2) (Math|Float|Lerp (.y (Variables|Default|GetChickenStartPos)) (.y _chickenendpos) _newtrack_2) (Math|Float|Lerp (Variables|Default|GetChickenHeight) (+ (Variables|Default|GetChickenHeight) 35.0) _newtrack_0)) true false))
      (:Finished
        (Variables|Default|SetChickenStartPos (Variables|Default|GetChickenEndPos))
        (Variables|Default|SetIsJumping false)
        (CallFunction|SetJumpableDirections)
        (if (Utilities|Array|IsValidIndex (Collision|GetOverlappingActors _capsule "/Game/BluePrints/BP_River.BP_River_C" :!class /Script/Engine.PrimitiveComponent))
          (Variables|Default|SetIsDoomed true)
          (bind _array_element (Utilities|Array|ForEachLoopwithBreak (Collision|GetOverlappingActors _capsule 0 :!class /Script/Engine.PrimitiveComponent))
            (:LoopBody
              (Utilities|Casting|CastToBP_Log _array_element
                (:then
                  _)
                (:CastFailed
                  (Utilities|Casting|CastToBP_Lilypad _array_element
                    (:then
                      _)
                    (:CastFailed
                      (Utilities|Casting|CastToBP_Road _array_element
                        (:then
                          _)
                        (:CastFailed
                          (Utilities|Casting|CastToBP_Railroad _array_element
                            (:then
                              _)
                            (:CastFailed
                              (Utilities|Casting|CastToBP_Grass _array_element)))))))))
              (Variables|Default|SetIsDoomed false))
            (:Completed
              (if (Variables|Default|GetIsDoomed)
                (Input|SetInputModeUIOnly (Game|GetPlayerController 0) 0 "DoNotLock")
                (Audio|PlaySound2D "/Game/Sounds/ChickenDeathKnell.ChickenDeathKnell" 1.0 1.0 0.0 0 0)
                (Audio|PlaySound2D "/Game/Sounds/rapidsdeath9.rapidsdeath9" 1.0 1.0 0.0 0 0)
                (Variables|Default|SetChickenHeight (.z _returnvalue_2))
                (bind _chickenheightpercentageduringdrowning (Timeline|ChickenDrowns Play)
                  (:Update
                    (Transformation|SetActorLocation (Math|Vector|MakeVector (.x _returnvalue_2) (.y _returnvalue_2) (Math|Float|Lerp (Variables|Default|GetChickenHeight) -25.0 _chickenheightpercentageduringdrowning)) false false))
                  (:Finished
                    (Effects|SpawnEmitteratLocation "/Game/Misc/PS_Drown.PS_Drown" (Math|Vector|MakeVector (.x _returnvalue_2) (.y _returnvalue_2) 3e+01))
                    (Transformation|SetWorldScale3D (Variables|Default|GetChickenMesh) "0, 0, 0")
                    (Utilities|FlowControl|Delay 3.0)
                    (CallFunction|KillChicken)
                    (Game|QuitGame 0 "Quit" false)))
                (else
                  (Timeline|Timeline_0 SetNewTime)))))
          (else
            (Timeline|Timeline_0 SetNewTime)))))
    (elif (or (== (Variables|Default|GetBackHops) 3) (<= (Variables|Default|GetTimeUntilEaten) 0.0))
      (Variables|Default|SetBackHops 0)
      (Variables|Default|SetTimeUntilEaten 15.0)
      (Game|SpawnActorfromClass "/Game/BluePrints/BP_Eagle.BP_Eagle_C" (Math|Transform|MakeTransform (Math|Vector|MakeVector (+ (.x _returnvalue) 8e+02) (.y _returnvalue) (+ (.z _returnvalue) 4e+02)) "0,-90.000000, 0" "1,1,1") "Undefined" 0 0)
      (Input|SetInputModeUIOnly (Game|GetPlayerController 0) 0 "DoNotLock")
      (Utilities|FlowControl|Delay 3.0)
      (CallFunction|KillChicken)
      (Game|QuitGame 0 "Quit" false)
      (else
        (bind _returnvalue_3 (Class|Pawn|ConsumeMovementInputVector))
        (Transformation|AddActorLocalOffset (* _returnvalue_3 DeltaSeconds) true false)
        (if (not (Math|Vector|VectorIsZero (Class|Pawn|GetLastMovementInputVector)))
          (Transformation|SetWorldRotation (Variables|Default|GetChickenMesh) (Math|Conversions|RotationFromXVector _returnvalue_3) false false))))))

(event Input|ActionEvents|InputActionHopForward
  (params (Key :type Key%20Structure :default "None"))
  (bind _returnvalue (Transformation|GetActorLocation))
  (:Pressed
    (if (not (Variables|Default|GetIsJumping))
      (if (Variables|Default|GetCanJumpForward)
        (Audio|PlaySound2D "/Game/Sounds/ChickenClucks.ChickenClucks" 1.0 1.0 0.0 0 0)
        (if (== (Variables|Default|GetBackHops) 0)
          (Variables|Default|SetTimeUntilEaten 15.0)
          (Variables|Default|SetFinalScore (+ (Variables|Default|GetFinalScore) 1))
          (else
            (Variables|Default|SetBackHops (- (Variables|Default|GetBackHops) 1))))
        (bind _output_get (Variables|Default|SetChickenStartPos (Transformation|GetActorLocation)))
        (Variables|Default|SetChickenEndPos (Math|Vector|MakeVector (+ (.x _output_get) (Variables|Default|GetChickenSpeed)) (.y _returnvalue) (.z _returnvalue)))
        (Variables|Default|SetIsJumping true)
        (Transformation|SetWorldRotation (Variables|Default|GetChickenMesh) (Math|Conversions|RotationFromXVector "200.000000, 0, 0") false false)
        (Variables|Default|SetCanJumpLeft true)
        (Variables|Default|SetCanJumpForward true)
        (Variables|Default|SetCanJumpBack true)
        (Variables|Default|SetCanJumpRight true)))))

(event Input|ActionEvents|InputActionHopRight
  (params (Key :type Key%20Structure :default "None"))
  (bind _returnvalue (Transformation|GetActorLocation))
  (:Pressed
    (if (not (Variables|Default|GetIsJumping))
      (if (Variables|Default|GetCanJumpRight)
        (Audio|PlaySound2D "/Game/Sounds/ChickenClucks.ChickenClucks" 1.0 1.0 0.0 0 0)
        (bind _output_get (Variables|Default|SetChickenStartPos (Transformation|GetActorLocation)))
        (Variables|Default|SetChickenEndPos (Math|Vector|MakeVector (.x _returnvalue) (+ (.y _output_get) (Variables|Default|GetChickenSpeed)) (.z _returnvalue)))
        (Variables|Default|SetIsJumping true)
        (Transformation|SetWorldRotation (Variables|Default|GetChickenMesh) (Math|Conversions|RotationFromXVector "0.000000,200.000000, 0") false false)
        (Variables|Default|SetCanJumpLeft true)
        (Variables|Default|SetCanJumpForward true)
        (Variables|Default|SetCanJumpBack true)
        (Variables|Default|SetCanJumpRight true)))))

(event Input|ActionEvents|InputActionHopLeft
  (params (Key :type Key%20Structure :default "None"))
  (bind _returnvalue (Transformation|GetActorLocation))
  (:Pressed
    (if (not (Variables|Default|GetIsJumping))
      (if (Variables|Default|GetCanJumpLeft)
        (Audio|PlaySound2D "/Game/Sounds/ChickenClucks.ChickenClucks" 1.0 1.0 0.0 0 0)
        (bind _output_get (Variables|Default|SetChickenStartPos (Transformation|GetActorLocation)))
        (Variables|Default|SetChickenEndPos (Math|Vector|MakeVector (.x _returnvalue) (+ (.y _output_get) (* -1 (Variables|Default|GetChickenSpeed))) (.z _returnvalue)))
        (Variables|Default|SetIsJumping true)
        (Transformation|SetWorldRotation (Variables|Default|GetChickenMesh) (Math|Conversions|RotationFromXVector "0.000000,-2.000000, 0") false false)
        (Variables|Default|SetCanJumpLeft true)
        (Variables|Default|SetCanJumpForward true)
        (Variables|Default|SetCanJumpBack true)
        (Variables|Default|SetCanJumpRight true)))))

(event Input|ActionEvents|InputActionHopBack
  (params (Key :type Key%20Structure :default "None"))
  (bind _returnvalue (Transformation|GetActorLocation))
  (:Pressed
    (if (not (Variables|Default|GetIsJumping))
      (if (Variables|Default|GetCanJumpBack)
        (Audio|PlaySound2D "/Game/Sounds/ChickenClucks.ChickenClucks" 1.0 1.0 0.0 0 0)
        (Variables|Default|SetBackHops (+ (Variables|Default|GetBackHops) 1))
        (bind _output_get (Variables|Default|SetChickenStartPos (Transformation|GetActorLocation)))
        (Variables|Default|SetChickenEndPos (Math|Vector|MakeVector (+ (.x _output_get) (* -1 (Variables|Default|GetChickenSpeed))) (.y _returnvalue) (.z _returnvalue)))
        (Variables|Default|SetIsJumping true)
        (Transformation|SetWorldRotation (Variables|Default|GetChickenMesh) (Math|Conversions|RotationFromXVector "-1.000000, 0, 0") false false)
        (Variables|Default|SetCanJumpLeft true)
        (Variables|Default|SetCanJumpForward true)
        (Variables|Default|SetCanJumpBack true)
        (Variables|Default|SetCanJumpRight true)))))

(event Input|AxisEvents|InputAxisMoveForward
  (params (AxisValue :type Float%20%28single-precision%29))
  ;[1 1 1] Continuous Movement
  (Pawn|Input|AddMovementInput (Transformation|GetActorForwardVector) (* AxisValue (* (Variables|Default|GetChickenSpeed) 1e+01)) false))

(event Input|AxisEvents|InputAxisMoveRight
  (params (AxisValue :type Float%20%28single-precision%29))
  ;[1 1 1] Continuous Movement
  (Pawn|Input|AddMovementInput (Transformation|GetActorRightVector) (* AxisValue (* (Variables|Default|GetChickenSpeed) 1e+01)) false))

(fn ConstructionScript)

(fn KillChicken
  (bind _mysave (Variables|Default|GetMySave))
  (bind _finalscore (Variables|Default|GetFinalScore))
  (if (> _finalscore (Variables|/Game/BluePrints/BP_Savegame.BP_Savegame_C|GetHighScore _mysave))
    (Variables|/Game/BluePrints/BP_Savegame.BP_Savegame_C|SetHighScore _mysave _finalscore))
  (Variables|/Game/BluePrints/BP_Savegame.BP_Savegame_C|SetTotalCoins _mysave (Variables|Default|GetCoinsCollected))
  (SaveGame|SaveGametoSlot _mysave "save"))

(fn SetJumpableDirections
  (bind _frontprobe (Variables|Default|GetFrontProbe))
  (bind _rightprobe (Variables|Default|GetRightProbe))
  (bind _backprobe (Variables|Default|GetBackProbe))
  (bind _leftprobe (Variables|Default|GetLeftProbe))
  (bind _overlappingactors (Collision|GetOverlappingActors _leftprobe 0 :!class /Script/Engine.PrimitiveComponent))
  (bind _overlappingactors_2 (Collision|GetOverlappingActors _frontprobe 0 :!class /Script/Engine.PrimitiveComponent))
  (bind _overlappingactors_3 (Collision|GetOverlappingActors _backprobe 0 :!class /Script/Engine.PrimitiveComponent))
  (bind _overlappingactors_4 (Collision|GetOverlappingActors _rightprobe 0 :!class /Script/Engine.PrimitiveComponent))
  (Utilities|FlowControl|Sequence
    (:then_0
      (if (Utilities|Array|IsValidIndex _overlappingactors_2)
        (for _array_element _overlappingactors_2
          (Utilities|Casting|CastToBP_Tree _array_element
            (:then
              _)
            (:CastFailed
              (Utilities|Casting|CastToBP_Rock _array_element)))
          (Variables|Default|SetCanJumpForward false))))
    (:then_1
      (if (Utilities|Array|IsValidIndex _overlappingactors_3)
        (for _array_element_2 _overlappingactors_3
          (Utilities|Casting|CastToBP_Tree _array_element_2
            (:then
              _)
            (:CastFailed
              (Utilities|Casting|CastToBP_Rock _array_element_2)))
          (Variables|Default|SetCanJumpBack false))))
    (:then_2
      (if (Utilities|Array|IsValidIndex _overlappingactors_4)
        (for _array_element_3 _overlappingactors_4
          (Utilities|Casting|CastToBP_Tree _array_element_3
            (:then
              _)
            (:CastFailed
              (Utilities|Casting|CastToBP_Rock _array_element_3)))
          (Variables|Default|SetCanJumpRight false)))
      (if (>= (.y (Transformation|GetActorLocation)) 1.49e+03)
        (Variables|Default|SetCanJumpRight false)))
    (:then_3
      (if (Utilities|Array|IsValidIndex _overlappingactors)
        (for _array_element_4 _overlappingactors
          (Utilities|Casting|CastToBP_Tree _array_element_4
            (:then
              _)
            (:CastFailed
              (Utilities|Casting|CastToBP_Rock _array_element_4)))
          (Variables|Default|SetCanJumpLeft false)))
      (if (<= (.y (Transformation|GetActorLocation)) -4.9e+02)
        (Variables|Default|SetCanJumpLeft false)))
    (:then_4
      (Default|UpdateUI (Variables|Default|GetMyHUD)))))