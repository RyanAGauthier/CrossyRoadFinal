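; Endless lane generator for a Crossy Road-style game, building random road, river, railroad and grass strips along X.
; RoadMaker runs at BeginPlay, randomizing each lane's type, direction and road or river contents through per-type spawn helpers.
; When the player overlaps the Box, the spawner jumps forward, destroys all but the most recent lanes, then spawns another batch.
; Spawned lanes accumulate in MyStuff; destroyed entries are never removed, only skipped by validity checks.
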(event OnComponentBeginOverlap(Box)
  (params (OverlappedComponent :type Primitive%20Component%20Object%20Reference) (OtherActor :type Actor%20Object%20Reference) (OtherComp :type Primitive%20Component%20Object%20Reference) (OtherBodyIndex :type Integer) (bFromSweep :type Boolean) (SweepResult :type Hit%20Result%20Structure%20%28by%20ref%29))
  (bind _mystuff (Variables|Default|GetMyStuff))
  (Utilities|Casting|CastToBP_Player OtherActor)
  (Transformation|AddActorLocalOffset (Math|Vector|MakeVector (* (Variables|Default|GetRoadsToSpawn) 1e+02) 0.0 0.0) false false)
  (for (_array_element _array_index) _mystuff
    (Utilities|IsValid _array_element
      (:Is%20Valid
        (if (< _array_index (- (Utilities|Array|LastIndex _mystuff) 15))
          (Actor|DestroyActor _array_element)))))
  (CallFunction|RoadMaker))

(event EventBeginPlay
  (CallFunction|RoadMaker))

(event Collision|EventActorBeginOverlap
  (params (OtherActor :type Actor%20Object%20Reference)))

(event EventTick
  (params (DeltaSeconds :type Float%20%28single-precision%29)))

(fn ConstructionScript)

(fn SpawnRoad
  (params (SpawnLocation :type Vector) (CarGap :type Float%20%28single-precision%29) (LaneSpeed :type Float%20%28single-precision%29) (Vehicle :type String) (RoadOrientation :type Rotator))
  (bind _output_get (LocalVariables|SetGapDetermination CarGap))
  (if (Utilities|Enum|Equal(Enum) Vehicle "Car")
    _
    (else
      (LocalVariables|SetGapDetermination (+ _output_get 2e+02))))
  (bind _returnvalue (Game|SpawnActorfromClass "/Game/BluePrints/BP_Road.BP_Road_C" (Math|Transform|MakeTransform SpawnLocation RoadOrientation "1,1,1") "Undefined" 0 (LocalVariables|GetGapDetermination) LaneSpeed Vehicle RoadOrientation 0))
  (return _returnvalue))

(fn RoadMaker
  (bind _returnvalue (Transformation|GetActorLocation))
  (bind _returnvalue_2 (Math|Random|RandomInteger 2))
  (bind _returnvalue_3 (Math|Random|RandomInteger 3))
  (bind _returnvalue_4 (* _returnvalue_2 1.8e+02))
  (bind _returnvalue_5 (> _returnvalue_3 0))
  (bind _returnvalue_6 (+ _returnvalue_4 -9e+01))
  (for _index (range 0 (Variables|Default|GetRoadsToSpawn))
    (switch int (Math|Random|RandomInteger 4)
      (:0
        (if _returnvalue_5
          (Variables|Default|SetVehicleToSpawn "Car")
          (else
            (Variables|Default|SetVehicleToSpawn "Truck")))
        (bind _output_get (Variables|Default|SetCurrentOrientation (Math|Rotator|MakeRotator 0.0 0.0 _returnvalue_6)))
        (if (== (.yaw _output_get) 9e+01)
          (Variables|Default|SetYOffset 0.0)
          (else
            (Variables|Default|SetYOffset 2e+03)))
        (bind _createdroad (CallFunction|SpawnRoad (Math|Vector|MakeVector (+ (.x _returnvalue) (* _index 9e+01)) (+ (.y _returnvalue) (Variables|Default|GetYOffset)) (.z _returnvalue)) (Math|Random|RandomFloatinRange 2e+02 6e+02) 9e+01 (Variables|Default|GetVehicleToSpawn) (Variables|Default|GetCurrentOrientation)))
        (Utilities|Array|Add (Variables|Default|GetMyStuff) _createdroad))
      (:1
        (if _returnvalue_5
          (Variables|Default|SetVehicleToSpawn "Lilypad")
          (Variables|Default|SetCurrentOrientation (Math|Rotator|MakeRotator 0.0 0.0 9e+01))
          (Variables|Default|SetYOffset 0.0)
          (else
            (Variables|Default|SetVehicleToSpawn "Log")
            (bind _output_get_2 (Variables|Default|SetCurrentOrientation (Math|Rotator|MakeRotator 0.0 0.0 _returnvalue_6)))
            (if (== (.yaw _output_get_2) 9e+01)
              (Variables|Default|SetYOffset 0.0)
              (else
                (Variables|Default|SetYOffset 2e+03)))))
        (bind _createdriver (CallFunction|SpawnRiver (Math|Vector|MakeVector (+ (.x _returnvalue) (* _index 9e+01)) (+ (.y _returnvalue) (Variables|Default|GetYOffset)) (- (.z _returnvalue) 1e+01)) (Variables|Default|GetVehicleToSpawn) (Variables|Default|GetCurrentOrientation)))
        (Utilities|Array|Add (Variables|Default|GetMyStuff) _createdriver))
      (:2
        (if _returnvalue_5
          (Variables|Default|SetCurrentOrientation (Math|Rotator|MakeRotator 0.0 0.0 9e+01))
          (Variables|Default|SetYOffset 0.0)
          (else
            (bind _output_get_3 (Variables|Default|SetCurrentOrientation (Math|Rotator|MakeRotator 0.0 0.0 _returnvalue_6)))
            (if (== (.yaw _output_get_3) 9e+01)
              (Variables|Default|SetYOffset 0.0)
              (else
                (Variables|Default|SetYOffset 2e+03)))))
        (bind _createdrailroad (CallFunction|SpawnRailroad (Math|Vector|MakeVector (+ (.x _returnvalue) (* _index 9e+01)) (+ (.y _returnvalue) (Variables|Default|GetYOffset)) (.z _returnvalue)) (Variables|Default|GetCurrentOrientation)))
        (Utilities|Array|Add (Variables|Default|GetMyStuff) _createdrailroad))
      (:3
        (Variables|Default|SetCurrentOrientation (Math|Rotator|MakeRotator 0.0 0.0 9e+01))
        (bind _createdgrass (CallFunction|SpawnGrass (Math|Vector|MakeVector (+ (.x _returnvalue) (* _index 9e+01)) (.y _returnvalue) (.z _returnvalue)) (Variables|Default|GetCurrentOrientation)))
        (Utilities|Array|Add (Variables|Default|GetMyStuff) _createdgrass)))))

(fn SpawnRiver
  (params (SpawnLocation :type Vector) (Entity :type String) (Orientation :type Rotator))
  (bind _returnvalue (Game|SpawnActorfromClass "/Game/BluePrints/BP_River.BP_River_C" (Math|Transform|MakeTransform SpawnLocation Orientation "1,1,1") "Undefined" 0 Entity 0))
  (return _returnvalue))

(fn SpawnRailroad
  (params (SpawnLocation :type Vector) (Orientation :type Rotator))
  (bind _returnvalue (Game|SpawnActorfromClass "/Game/BluePrints/BP_RailRoad.BP_Railroad_C" (Math|Transform|MakeTransform SpawnLocation Orientation "1,1,1") "Undefined" 0 0))
  (return _returnvalue))

(fn SpawnGrass
  (params (SpawnLocation :type Vector) (Orientation :type Rotator))
  (bind _returnvalue (Game|SpawnActorfromClass "/Game/BluePrints/BP_Grass.BP_Grass_C" (Math|Transform|MakeTransform SpawnLocation Orientation "1,1,1") "Undefined" 0 0))
  (return _returnvalue))