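; BP_Playerchar is the player character, a chicken that moves in hops along the world X and Y axes.
; Four Hop input actions call LaunchCharacter using ChickenSpeed and LaunchHeight, overriding current velocity, then turn the static mesh to face the hop direction.
; Left, right and back hops are blocked while falling, but forward hop has no such check.
; MoveForward and MoveRight axis events are empty, with their AddMovementInput logic left disconnected.
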(event EventBeginPlay)

(event Collision|EventActorBeginOverlap
  (params (OtherActor :type Actor%20Object%20Reference)))

(event EventTick
  (params (DeltaSeconds :type Float%20%28single-precision%29)))

(event Input|ActionEvents|InputActionHopForward
  (params (Key :type Key%20Structure :default "None"))
  (:Pressed
    (Character|LaunchCharacter (Math|Vector|MakeVector (Variables|Default|GetChickenSpeed) 0.0 (Variables|Default|GetLaunchHeight)) true true)
    (Transformation|SetWorldRotation (Variables|Default|GetStaticMesh) (Math|Conversions|RotationFromXVector "1.000000,0.000000, 0") false false)))

(event Input|ActionEvents|InputActionHopRight
  (params (Key :type Key%20Structure :default "None"))
  (:Pressed
    (if (not (AI|Components|NavMovement|IsFalling (Variables|Character|GetCharacterMovement)))
      (Character|LaunchCharacter (Math|Vector|MakeVector 0.0 (Variables|Default|GetChickenSpeed) (Variables|Default|GetLaunchHeight)) true true)
      (Transformation|SetWorldRotation (Variables|Default|GetStaticMesh) (Math|Conversions|RotationFromXVector "0.000000,10.000000, 0") false false))))

(event Input|ActionEvents|InputActionHopBack
  (params (Key :type Key%20Structure :default "None"))
  (:Pressed
    (if (not (AI|Components|NavMovement|IsFalling (Variables|Character|GetCharacterMovement)))
      (Character|LaunchCharacter (Math|Vector|MakeVector (* -1 (Variables|Default|GetChickenSpeed)) 0.0 (Variables|Default|GetLaunchHeight)) true true)
      (Transformation|SetWorldRotation (Variables|Default|GetStaticMesh) (Math|Conversions|RotationFromXVector "-1.000000,0.000000,0.000000") false false))))

(event Input|ActionEvents|InputActionHopLeft
  (params (Key :type Key%20Structure :default "None"))
  (:Pressed
    (if (not (AI|Components|NavMovement|IsFalling (Variables|Character|GetCharacterMovement)))
      (Character|LaunchCharacter (Math|Vector|MakeVector 0.0 (* -1 (Variables|Default|GetChickenSpeed)) (Variables|Default|GetLaunchHeight)) true true)
      (Transformation|SetWorldRotation (Variables|Default|GetStaticMesh) (Math|Conversions|RotationFromXVector "0.000000,-10.000000, 0") false false))))

(event Input|AxisEvents|InputAxisMoveForward
  (params (AxisValue :type Float%20%28single-precision%29)))

(event Input|AxisEvents|InputAxisMoveRight
  (params (AxisValue :type Float%20%28single-precision%29)))

(fn ConstructionScript)